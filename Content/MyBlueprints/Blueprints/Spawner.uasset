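; Spawner actor that assembles a level at BeginPlay from randomly chosen obstacle sections.
; It loads one of six obstacle sublevels as a level instance for each step of LevelLength, offset by Distance from the actor's location.
; After the last section it spawns an end actor selected by CurrentLevel, either a transition to the next level or the final End.
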(event `self.ReceiveBeginPlay`
  (for _index (range (`self.LevelLength`))
    (`LevelStreamingDynamic.LoadLevelInstanceBySoftObjectPtr` (select `int` (`KismetMathLibrary.RandomIntegerInRange` 0 5) :`0` "/Game/MyBlueprints/Obstacles/Obstacle1.Obstacle1" :`1` "/Game/MyBlueprints/Obstacles/Obstacle2.Obstacle2" :`2` "/Game/MyBlueprints/Obstacles/Obstacle3.Obstacle3" :`3` "/Game/MyBlueprints/Obstacles/Obstacle4.Obstacle4" :`4` "/Game/MyBlueprints/Obstacles/Obstacle5.Obstacle5" :`5` "/Game/MyBlueprints/Obstacles/Obstacle6.Obstacle6" :!type "World Soft Object Reference") (+ (`self.K2_GetActorLocation`) (* (`self.Distance`) _index))))
  (`|SpawnActorFromClass` (select `int` (- (`self.CurrentLevel`) 1) :`0` "/Game/MyBlueprints/Blueprints/ToLevel2.ToLevel2_C" :`1` "/Game/MyBlueprints/Blueprints/ToLevel3.ToLevel3_C" :`2` "/Game/MyBlueprints/Blueprints/ToLevel4.ToLevel4_C" :`3` "/Game/MyBlueprints/Blueprints/End.End_C" :!type "Actor Class Reference") (`KismetMathLibrary.MakeTransform` (+ (`self.K2_GetActorLocation`) (* (`self.Distance`) (`self.LevelLength`)))) "Undefined" "OverrideRootScale"))

(fn `UserConstructionScript`)